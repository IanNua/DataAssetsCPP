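; BP_FantasyVillager is a villager actor that configures its appearance and info display from its MPDA variable, which supplies race and villager data.
; On BeginPlay it tints the cube through a dynamic instance of M_RaceBase, scales it to the character size and shows the race name on a TextRender.
; It then passes the villager's name and health to the W_VillagerInfo widget in the Stats component.
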(event EventBeginPlay
  (bind _self self)
  (bind _mpda (Variables|Default|GetMPDA))
  (bind _stats (Variables|Default|GetStats))
  (bind _returnvalue (Transformation|GetActorTransform _self))
  (bind _returnvalue_2 (UserInterface|GetWidget _stats))
  (bind _asw_villager_info (Utilities|Casting|CastToW_VillagerInfo _returnvalue_2))
  (bind _returnvalue_3 (Rendering|Material|CreateDynamicMaterialInstance (Variables|Default|GetCube) 0 "/Game/M_RaceBase.M_RaceBase" "None" :!class /Script/Engine.PrimitiveComponent))
  (Rendering|Material|SetVectorParameterValue _returnvalue_3 "MatColour" (Math|Conversions|ToLinearColor(Color) (Variables|/Script/C.MyPrimaryDataAsset|GetmaterialColour _mpda)) :!class /Script/Engine.MaterialInstanceDynamic)
  (Rendering|Components|TextRender|SetText (Variables|Default|GetTextRender) (Utilities|Text|ToText(String) (Variables|/Script/C.MyPrimaryDataAsset|GetfantasyRaceName _mpda)))
  (Transformation|SetWorldTransform (Variables|Default|GetCube) (Math|Transform|MakeTransform (.location _returnvalue) (.rotation _returnvalue) (Variables|/Script/C.MyPrimaryDataAsset|GetSizeofCharacter _mpda)) false false)
  (UserInterface|SetWidget (Variables|Default|GetStats) _returnvalue_2)
  (Variables|/Game/W_VillagerInfo.W_VillagerInfo_C|SetVillagerName _asw_villager_info (Utilities|Text|ToText(String) (Variables|/Script/C.MyPrimaryDataAsset|GetvillagerName _mpda)))
  (Variables|/Game/W_VillagerInfo.W_VillagerInfo_C|SetVillagerHealth _asw_villager_info (Variables|/Script/C.MyPrimaryDataAsset|GetvillagerHealth _mpda)))

(event Collision|EventActorBeginOverlap
  (params (OtherActor :type Actor%20Object%20Reference)))

(event EventTick
  (params (DeltaSeconds :type Float%20%28single-precision%29)))

(fn ConstructionScript)